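; BP_CamerasEnjoyer keeps a scene capture camera mirroring the player's main camera at a large fixed X offset, apparently to render a second, distant copy of the level.
; On BeginPlay it caches the third-person character and the capture component of a SceneCapture2D found in the level.
; Each Tick, moved to the post-update-work group, teleports that component to the main camera's offset transform, preserving rotation and scale.
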(event `self.ReceiveBeginPlay`
  (`self.SetTickGroup` "TG_PostUpdateWork")
  (bind _asbp_third_person_character (cast `/Game/ThirdPerson/Blueprints/BP_ThirdPersonCharacter` (`GameplayStatics.GetPlayerPawn` 0)))
  (set `self.PlayerCharacter` _asbp_third_person_character)
  (bind _returnvalue (`GameplayStatics.GetActorOfClass` "/Script/Engine.SceneCapture2D"))
  (set `self.SecondaryCamera` (`SceneCapture2D.CaptureComponent2D` _returnvalue)))

(event `self.ReceiveTick`
  (params (DeltaSeconds :type "Float (single-precision)"))
  (bind _maincamera (`/Game/ThirdPerson/Blueprints/BP_ThirdPersonCharacter.MainCamera` (`self.PlayerCharacter`)))
  (`CameraComponent.GetCameraView` _maincamera 0.0)
  (`SceneComponent.K2_SetWorldTransform` (`self.SecondaryCamera`) (`KismetMathLibrary.MakeTransform` (+ (100000.0 0.0 0.0) (.location (`SceneComponent.K2_GetComponentToWorld` _maincamera))) (.rotation (`SceneComponent.K2_GetComponentToWorld` _maincamera)) (.scale (`SceneComponent.K2_GetComponentToWorld` _maincamera))) false true))

(fn `UserConstructionScript`)