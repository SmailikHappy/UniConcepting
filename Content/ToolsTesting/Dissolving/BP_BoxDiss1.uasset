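; Test box actor that defines a dissolve volume for materials through the MPC_DissMat1 parameter collection.
; Its construction script writes the Cube's world location, scale and forward, right and up vectors into the collection, so the values are not updated at runtime.
; When a sphere component of a SimpleActor begins overlapping the Cube, it calls SphereTriggered on that actor with the sphere, printing debug strings along the way.
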(event `self.Cube.OnComponentBeginOverlap`
  (params (OverlappedComponent :type "PrimitiveComponent Object Reference") (OtherActor :type "Actor Object Reference") (OtherComp :type "PrimitiveComponent Object Reference") (OtherBodyIndex :type Integer) (bFromSweep :type Boolean) (SweepResult :type "HitResult Structure (by ref)"))
  (bind _assimple_actor (cast `/Game/ToolsTesting/UnnecessaryFolder/SimpleActor` OtherActor)
    (:`then`
      (bind _assphere_collision (cast `SphereComponent` OtherComp)
        (:`then`
          (`KismetSystemLibrary.PrintString` "Hello")
          (`/Game/ToolsTesting/UnnecessaryFolder/SimpleActor.SphereTriggered` _assimple_actor _assphere_collision))
        (:`CastFailed`
          (`KismetSystemLibrary.PrintString` "Wrong component"))))
    (:`CastFailed`
      (`KismetSystemLibrary.PrintString` "Wrong actor"))))

(fn `UserConstructionScript`
  (`KismetMaterialLibrary.SetVectorParameterValue` "/Game/ToolsTesting/Dissolving/MPC_DissMat1.MPC_DissMat1" "Location" (`KismetMathLibrary.Conv_VectorToLinearColor` (`SceneComponent.K2_GetComponentLocation` (`self.Cube`))))
  (`KismetMaterialLibrary.SetVectorParameterValue` "/Game/ToolsTesting/Dissolving/MPC_DissMat1.MPC_DissMat1" "Scale" (`KismetMathLibrary.Conv_VectorToLinearColor` (`SceneComponent.K2_GetComponentScale` (`self.Cube`))))
  (`KismetMaterialLibrary.SetVectorParameterValue` "/Game/ToolsTesting/Dissolving/MPC_DissMat1.MPC_DissMat1" "XRot (forward)" (`KismetMathLibrary.Conv_VectorToLinearColor` (`SceneComponent.GetForwardVector` (`self.Cube`))))
  (`KismetMaterialLibrary.SetVectorParameterValue` "/Game/ToolsTesting/Dissolving/MPC_DissMat1.MPC_DissMat1" "YRot (right)" (`KismetMathLibrary.Conv_VectorToLinearColor` (`SceneComponent.GetRightVector` (`self.Cube`))))
  (`KismetMaterialLibrary.SetVectorParameterValue` "/Game/ToolsTesting/Dissolving/MPC_DissMat1.MPC_DissMat1" "ZRot (up)" (`KismetMathLibrary.Conv_VectorToLinearColor` (`SceneComponent.GetUpVector` (`self.Cube`)))))