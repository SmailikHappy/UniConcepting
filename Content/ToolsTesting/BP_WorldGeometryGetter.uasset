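; Function library that finds the world geometry cache for slime mold tooling and reports errors from editor tools.
; GetWorldGeometryForSlimeMold searches the level for BP_WorldGeometryCache actors and returns the first, logging when several exist or returning empty with a log when none do.
; HandleToolError shows a message as a user warning on the given tool and adds it to that tool's log as highlighted.
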(fn `GetWorldGeometryForSlimeMold`
  (params (WorldContext :type "Object Object Reference"))
  (returns (WorldGeometryCache :type "/Game/ToolsTesting/BP_WorldGeometryCache Object Reference"))
  (bind _outactors (`GameplayStatics.GetAllActorsOfClass` WorldContext "/Game/ToolsTesting/BP_WorldGeometryCache.BP_WorldGeometryCache_C"))
  (bind _returnvalue (`KismetArrayLibrary.Array_Length` _outactors))
  (if (== _returnvalue 1)
    _
    (elif (!= _returnvalue 0)
      (`KismetSystemLibrary.LogString` "There is more then 1 Geometry Cache in the level, taking the first one")
      (else
        (`KismetSystemLibrary.LogString` "There is no Geometry Cache in the level")
        (return null))))
  (return (`|GetArrayItem` _outactors)))

(fn `HandleToolError`
  (params (Tool :type "ScriptableInteractiveTool Object Reference") (Message :type Text))
  (`ScriptableInteractiveTool.DisplayUserWarningMessage` Tool Message)
  (`ScriptableInteractiveTool.AddLogMessage` Tool Message true))