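; Editor-style goop generator that builds a slime-mold dynamic mesh over surrounding geometry, driven by SlimeMoldSkeleton custom buttons.
; Caching merges SurroundingMeshes into one BVH-backed mesh, whose nearest-point queries guide seeded, jittered splines along skeleton lines.
; Generation sweeps these into thickness-scaled tubes, or draws debug lines, and grows veinness-driven branch splines that are not meshed.
; Separate buttons apply SDF-morphology retopology with tessellation, smoothing and UVs, or assign material.
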(event `self.SlimeMoldSkeleton.OnCustomButtonPress`
  (params (Properties :type "Object Object Reference") (Key :type String))
  (bind _asps_goop_properties (cast `/Game/ToolsTesting/NewGeneration/PS_GoopProperties` Properties)
    (:`then`
      (switch `string` Key
        (:`Default`
          (`KismetSystemLibrary.PrintString` (`KismetStringLibrary.Concat_StrStr` "Unknown key received: " Key) true true (struct :`R` 1.0 :`B` 0.11875 :`A` 1.0)))
        (:`GenerateMesh`
          (`self.ClearMesh`)
          (`self.GenerateMesh` _asps_goop_properties))
        (:`GenerateDebug`
          (`self.ClearMesh`)
          (`self.GenerateMesh` _asps_goop_properties true))
        (:`Retopology`
          (`self.ApplyRetopology` _asps_goop_properties))
        (:`Material`
          (`self.ApplyMaterial` _asps_goop_properties))
        (:`ClearMesh`
          (`self.ClearMesh`))
        (:`CacheSurrondingGeoemtry`
          (`self.CacheSurroundingGeometry` _asps_goop_properties))
        (:`HideSurrondingGeoemtry`
          (`self.SetVisibilityOfSurroundingGeometry` false))
        (:`ShowSurrondingGeoemtry`
          (`self.SetVisibilityOfSurroundingGeometry` true))))
    (:`CastFailed`
      (`KismetSystemLibrary.PrintString` "Property cast failed" true true (struct :`R` 1.0 :`B` 0.11875 :`A` 1.0)))))

(fn `# F Grow Splines from Base Spline`
  (params (SourceSpline :type "SplineComponent Object Reference") (BaseSplineInfo :type "/Game/ToolsTesting/UnnecessaryFolder/S_SMBranchData Structure") (NewSplineGenerationInfo :type "/Game/ToolsTesting/UnnecessaryFolder/S_SMBranchGenerationInfo Structure"))
  (returns (NewSplines :type "Array of SplineComponent Object Reference"))
  (locals (MinVeinness :type "Float (double-precision)") (MaxVeinness :type "Float (double-precision)") (Splines :type "Array of SplineComponent Object Reference") (Stream :type "RandomStream Structure" :default (struct :`InitialSeed` 3)) (RandomDistance :type "Float (double-precision)") (TempPointsForNewSpline :type "Array of Vector Structure") (NewSplineOriginScale :type "Vector Structure") (TempStepForNewSpline :type "Float (double-precision)"))
  (bind ((`BeginVeinness_21_09793C174D5CB7AE6AE4CEA23B64A43F` _beginveinness) (`EndVeinness_23_DB7515C24C5F30B8511F1FBBCAB64344` _endveinness)) (break `/Game/ToolsTesting/UnnecessaryFolder/S_SMBranchData` BaseSplineInfo))
  (bind (_minrandomlength _maxrandomlength _mindistancetogrowfrom _step) (break `/Game/ToolsTesting/UnnecessaryFolder/S_SMBranchGenerationInfo` NewSplineGenerationInfo))
  (bind ((`ConeHalfAngle_20_FDB1C1E8432E07D8466A15939EEA0B79` _conehalfangle) (`InitialMaxOffsetAngle_34_6967DCB246C1AA3294978E93093196A6` _initialmaxoffsetangle)) (break `/Game/ToolsTesting/UnnecessaryFolder/S_SMBranchGenerationInfo` NewSplineGenerationInfo))
  (bind _newsplineoriginscale (`local.NewSplineOriginScale`))
  (bind _stream (`local.Stream`))
  (bind _temppointsfornewspline (`local.TempPointsForNewSpline`))
  (bind _returnvalue (`KismetMathLibrary.RandomFloatInRangeFromStream` (`local.Stream`) _minrandomlength _maxrandomlength))
  (bind _output (`|GetArrayItem` (`local.TempPointsForNewSpline`)))
  (bind _returnvalue_2 (`KismetMathLibrary.FFloor` (/ _returnvalue _step)))
  (set `local.MinVeinness` (`KismetMathLibrary.FMin` _beginveinness _endveinness))
  (bind _output_get (set `local.MaxVeinness` (`KismetMathLibrary.FMax` _beginveinness _endveinness)))
  (for _index (range 1 (+ (`KismetMathLibrary.FFloor` _output_get) 1))
    (bind _returnvalue_3 (`KismetMathLibrary.Conv_IntToDouble` _index))
    (if (<= _returnvalue_3 (`local.MaxVeinness`))
      (bind _returnvalue_4 (`KismetMathLibrary.FClamp` (/ (- _returnvalue_3 (`local.MinVeinness`)) (`KismetMathLibrary.FMax` (- (`local.MaxVeinness`) (`local.MinVeinness`)) 0.0001))))
      (bind _output_get_2 (set `local.RandomDistance` (* (`SplineComponent.GetSplineLength` SourceSpline) (`KismetMathLibrary.SelectFloat` (`KismetMathLibrary.RandomFloatInRangeFromStream` _stream _returnvalue_4 1.0) (`KismetMathLibrary.RandomFloatInRangeFromStream` _stream 0.0 (- 1.0 _returnvalue_4)) (== _beginveinness (`local.MinVeinness`))))))
      ;[1 1 1] Get the initial direction that is more / less perpendicular to base spline
      (`KismetArrayLibrary.Array_Add` (`local.TempPointsForNewSpline`) (`SplineComponent.GetLocationAtDistanceAlongSpline` SourceSpline _output_get_2 "World"))
      (set `local.NewSplineOriginScale` (`SplineComponent.GetScaleAtDistanceAlongSpline` SourceSpline _output_get_2))
      (set `local.TempStepForNewSpline` (/ _returnvalue _returnvalue_2))
      (bind (_nearestresult _returnvalue_5) (`GeometryScriptLibrary_MeshSpatial.FindNearestPointOnMesh` (`self.SurroundingsRaycastMesh`) (`self.SurroundingsRaycastBVH`) _output (struct) null)
        (:`Found`
          (bind (_bisvalidtriangle _returnvalue_6) (`GeometryScriptLibrary_MeshQueryFunctions.GetTriangleFaceNormal` _returnvalue_5 (`.TriangleID` (break `GeometryScriptTrianglePoint` _nearestresult))))
          (if _bisvalidtriangle
            (bind _nextpoint (`self.GetNextPoint` (* (`KismetMathLibrary.Cross_VectorVector` _returnvalue_6 (`SplineComponent.GetTangentAtDistanceAlongSpline` SourceSpline _output_get_2 "World")) (`KismetMathLibrary.SignOfFloat` (- (`KismetMathLibrary.Conv_BoolToDouble` (`KismetMathLibrary.RandomBoolFromStream` (`local.Stream`))) 0.5))) _output (`local.TempStepForNewSpline`) _initialmaxoffsetangle))
            (`KismetArrayLibrary.Array_Add` (`local.TempPointsForNewSpline`) _nextpoint)
            (else
              ;[1 1 1] If the initial direction is impossible to find, just use the random one (SHOULD NOT BE THE CASE, BUT IT IS HERE)
              (`KismetSystemLibrary.LogString` "[GEN ERROR] Normal of parsed triangle is not valid :?")
              (bind _nextpoint_2 (`self.GetNextPoint` (`KismetMathLibrary.RandomUnitVectorFromStream` (`local.Stream`)) _output (`local.TempStepForNewSpline`) _conehalfangle :!label _label))
              (`KismetArrayLibrary.Array_Add` (`local.TempPointsForNewSpline`) _nextpoint_2))))
        (:`NotFound`
          (`KismetSystemLibrary.LogString` "[GEN ERROR] Cant find a surface to grow")
          (goto _label)))
      ;[1 1 1] Generating the rest of the spline points
      (for _index_2 (range 1 (+ _returnvalue_2 1))
        (bind _output_2 (`|GetArrayItem` _temppointsfornewspline _index_2))
        (bind _nextpoint_3 (`self.GetNextPoint` (`KismetMathLibrary.Normal` (- _output_2 (`|GetArrayItem` _temppointsfornewspline (- _index_2 1)))) _output_2 (`local.TempStepForNewSpline`) _conehalfangle))
        (`KismetArrayLibrary.Array_Add` (`local.TempPointsForNewSpline`) _nextpoint_3))
      ;[1 1 1] Contructing the spline from points
      (bind _returnvalue_7 (`AddComponent|NODE_AddSplineComponent-5`))
      (`SplineComponent.SetSplinePoints` _returnvalue_7 (`local.TempPointsForNewSpline`) "World" true)
      (bind _returnvalue_8 (- (`SplineComponent.GetNumberOfSplinePoints` _returnvalue_7) 1))
      (for _index_3 (range (+ _returnvalue_8 1))
        (`SplineComponent.SetScaleAtSplinePoint` _returnvalue_7 _index_3 (`KismetMathLibrary.VLerp` _newsplineoriginscale (/ _newsplineoriginscale 2.0) (/ _index_3 _returnvalue_8)) true))
      (`KismetArrayLibrary.Array_Add` (`local.Splines`) _returnvalue_7)
      (`KismetArrayLibrary.Array_Clear` (`local.TempPointsForNewSpline`))))
  (return (`local.Splines`)))

(fn `ApplyMaterial`
  (params (Properties :type "/Game/ToolsTesting/NewGeneration/PS_GoopProperties Object Reference"))
  (`DynamicMeshComponent.ConfigureMaterialSet` (`self.DynamicMeshComponent`) (`|MakeArray` (`/Game/ToolsTesting/NewGeneration/PS_GoopProperties.Material` Properties) :!type "MaterialInterface Object Reference")))

(fn `ApplyRetopology`
  (params (Properties :type "/Game/ToolsTesting/NewGeneration/PS_GoopProperties Object Reference"))
  (bind _returnvalue (`GeometryScriptLibrary_MeshVoxelFunctions.ApplyMeshMorphology` (`self.TargetMesh`) (make `GeometryScriptMorphologyOptions` (make `GeometryScript3DGridParameters` "GridCellSize" (`/Game/ToolsTesting/NewGeneration/PS_GoopProperties.SDFGridCellSize` Properties)) false (make `GeometryScript3DGridParameters` "GridResolution") "Dilate" (`/Game/ToolsTesting/NewGeneration/PS_GoopProperties.ExtraThickness` Properties)) null))
  (bind _returnvalue_2 (`GeometryScriptLibrary_MeshSubdivideFunctions.ApplyPNTessellation` _returnvalue (make `GeometryScriptPNTessellateOptions` true) (`/Game/ToolsTesting/NewGeneration/PS_GoopProperties.Teselation` Properties) null))
  (bind _returnvalue_3 (`GeometryScriptLibrary_MeshDeformFunctions.ApplyIterativeSmoothingToMesh` _returnvalue_2 (struct) (make `GeometryScriptIterativeMeshSmoothingOptions` (`/Game/ToolsTesting/NewGeneration/PS_GoopProperties.SmoothIterations` Properties) (`/Game/ToolsTesting/NewGeneration/PS_GoopProperties.SmoothAlpha` Properties)) null))
  (bind _returnvalue_4 (`GeometryScriptLibrary_MeshUVFunctions.SetMeshUVsFromPlanarProjection` _returnvalue_3 0 (`KismetMathLibrary.MakeTransform` (0.0 0.0 0.0) (struct) (`KismetMathLibrary.Conv_DoubleToVector` (`KismetMathLibrary.FMax` (.x (`KismetMathLibrary.GetBoxSize` (`GeometryScriptLibrary_MeshQueryFunctions.GetMeshBoundingBox` _returnvalue_3))) (.y (`KismetMathLibrary.GetBoxSize` (`GeometryScriptLibrary_MeshQueryFunctions.GetMeshBoundingBox` _returnvalue_3)))))) (struct) null))
  (bind _returnvalue_5 (`GeometryScriptLibrary_MeshNormalsFunctions.ComputeTangents` _returnvalue_4 (struct) null))
  (`GeometryScriptLibrary_MeshNormalsFunctions.ComputeSplitNormals` _returnvalue_5 (make `GeometryScriptSplitNormalsOptions` true 80.0) (struct) null))

(fn `CacheSurroundingGeometry`
  (params (Properties :type "/Game/ToolsTesting/NewGeneration/PS_GoopProperties Object Reference"))
  (locals (MaxPointWorldLocation :type "Vector Structure") (MinPointWorldLocation :type "Vector Structure") (MaxActorWorldBounds :type "Vector Structure") (MinActorWorldBounds :type "Vector Structure"))
  (`|ExecutionSequence`
    (:`then_0`
      ;[1 1 1] Setting default variables
      (set `local.MaxPointWorldLocation` (-999999.0 -999999.0 -999999.0))
      (set `local.MinPointWorldLocation` (999999.0 999999.0 999990.0)))
    (:`then_3`
      ;[0.7636 0.7292 1 1 32] Putting all the meshes into a single mesh to raycast
      (`self.ReleaseComputeMesh` (`self.SurroundingsRaycastMesh`))
      (bind _returnvalue (`self.AllocateComputeMesh`))
      (set `self.SurroundingsRaycastMesh` _returnvalue)
      (for _array_element (`self.SurroundingMeshes`)
        (bind _returnvalue_2 (`self.AllocateComputeMesh`))
        (`|ExecutionSequence`
          (:`then_0`
            (bind (_localtoworld _returnvalue_3) (`GeometryScriptLibrary_SceneUtilityFunctions.CopyMeshFromComponent` (`Actor.RootComponent` _array_element) _returnvalue_2 (struct) false null)
              (:`Success`
                (`GeometryScriptLibrary_MeshBasicEditFunctions.AppendMesh` (`self.SurroundingsRaycastMesh`) _returnvalue_3 _localtoworld false (struct :`CombineMode` "EnableAllMatching") null))))
          (:`then_1`
            (`self.ReleaseComputeMesh` _returnvalue_2))))
      ;;[1 0.439 0.5799] Building BVH
      (bind _outputbvh (`GeometryScriptLibrary_MeshSpatial.BuildBVHForMesh` (`self.SurroundingsRaycastMesh`) null))
      (set `self.SurroundingsRaycastBVH` _outputbvh))))

(fn `ClearMesh`
  (bind (_triangleidlist _bhastriangleidgaps _returnvalue) (`GeometryScriptLibrary_MeshQueryFunctions.GetAllTriangleIDs` (`self.TargetMesh`)))
  (bind (_numdeleted _returnvalue_2) (`GeometryScriptLibrary_MeshBasicEditFunctions.DeleteTrianglesFromMesh` _returnvalue _triangleidlist))
  (`DynamicMesh.Reset` _returnvalue_2)
  (`KismetSystemLibrary.FlushPersistentDebugLines`))

(fn `DrawDebugLineIf`
  (params (DrawIfTrue :type Boolean) (LineStart :type "Vector Structure") (LineEnd :type "Vector Structure") (LineColor :type "LinearColor Structure") (Duration :type "Float (single-precision)") (Thickness :type "Float (single-precision)"))
  (if DrawIfTrue
    (`KismetSystemLibrary.DrawDebugLine` LineStart LineEnd LineColor Duration Thickness)))

(fn `GenerateMesh`
  (params (Properties :type "/Game/ToolsTesting/NewGeneration/PS_GoopProperties Object Reference") (DebugOutput :type Boolean))
  (bind _skeletonpoints (`SlimeMoldSkeletonComponent.SkeletonPoints` (`self.SlimeMoldSkeleton`)))
  (`|ExecutionSequence`
    (:`then_0`
      ;[1 0.6927 0.8464 1 32] Base splines
      (for (_array_element _array_index) (`SlimeMoldSkeletonComponent.SkeletonLines` (`self.SlimeMoldSkeleton`))
        (bind _output (`|GetArrayItem` _skeletonpoints (break `SkeletonLine` _array_element)))
        (bind _output_2 (`|GetArrayItem` _skeletonpoints (`.Point2ID` (break `SkeletonLine` _array_element))))
        (bind _basespline (`self.MakeBaseSpline2` _output _output_2 _array_index 20.0 4.0 0.5 (`local.DebugOutput`)))
        (`|ExecutionSequence`
          (:`then_0`
            (if (not (`local.DebugOutput`))
              (bind _resultingmesh (`self.MakeMeshFromSpline` _basespline))
              (`GeometryScriptLibrary_MeshBasicEditFunctions.AppendMesh` (`self.TargetMesh`) _resultingmesh (struct) false (struct :`CombineMode` "EnableAllMatching") null)))
          (:`then_1`
            (`KismetArrayLibrary.Array_Add` (`self.1stGenSplines`) _basespline)
            (bind (_relativepos _thickness _clusterization _veinness) (break `SkeletonPoint` _output))
            (bind (_relativepos_2 _thickness_2 _clusterization_2 _veinness_2) (break `SkeletonPoint` _output_2))
            (`self.# F Grow Splines from Base Spline` _basespline (make `/Game/ToolsTesting/UnnecessaryFolder/S_SMBranchData` _thickness _thickness_2 _clusterization _clusterization_2 _veinness _veinness_2) (make `/Game/ToolsTesting/UnnecessaryFolder/S_SMBranchGenerationInfo` 40.0 100.0 0.5))))))
    (:`then_2`
      ;[0 0 0 0] Updating transform
      (`GeometryScriptLibrary_MeshTransformFunctions.TransformMesh` (`self.TargetMesh`) (`KismetMathLibrary.InvertTransform` (`self.GetTransform`)) true null)
      (for _array_element_2 (`self.1stGenSplines`)
        (`ActorComponent.K2_DestroyComponent` _array_element_2)))))

(fn `GetNextPoint`
  (params (Direction :type "Vector Structure") (OriginPoint :type "Vector Structure") (`Preferred distance` :type "Float (double-precision)") (MaxRandomAngleOffset :type "Float (double-precision)"))
  (returns (NextPoint :type "Vector Structure") (`Nearest Polint On Mesh Position` :type "Vector Structure"))
  (locals (QueryPoint :type "Vector Structure") (Stream :type "RandomStream Structure"))
  (bind _output_get (set `local.QueryPoint` (+ OriginPoint (* `Preferred distance` (`KismetMathLibrary.RandomUnitVectorInConeInDegreesFromStream` (`local.Stream`) Direction MaxRandomAngleOffset)))))
  (bind _nearestresult (`GeometryScriptLibrary_MeshSpatial.FindNearestPointOnMesh` (`self.SurroundingsRaycastMesh`) (`self.SurroundingsRaycastBVH`) _output_get (struct) null)
    (:`Found`
      (return (+ (* `Preferred distance` (`KismetMathLibrary.Normal` (- (`.Position` (break `GeometryScriptTrianglePoint` _nearestresult)) OriginPoint))) OriginPoint) (0.0 0.0 0.0)))
    (:`NotFound`
      (`KismetSystemLibrary.PrintString` "Mesh get closest point failed" true true (struct :`R` 1.0 :`G` 0.015156 :`A` 1.0))
      (return (+ OriginPoint (`local.QueryPoint`)) (0.0 0.0 0.0)))))

(fn `MakeBaseSpline2`
  (params (SkeletonPoint1 :type "SkeletonPoint Structure (by ref)") (SkeletonPoint2 :type "SkeletonPoint Structure (by ref)") (StreamSeed :type Integer) (MainStep :type "Float (double-precision)" :default 20.0) (SubStep :type "Float (double-precision)" :default 4.0) (Gravity :type "Float (double-precision)" :default 0.5) (DebugDraw :type Boolean))
  (returns (BaseSpline :type "SplineComponent Object Reference"))
  (locals (Direction :type "Vector Structure") (Stream :type "RandomStream Structure") (TempClosestPointNormal :type "Vector Structure") (MaxDistanceToMesh :type "Float (double-precision)" :default 120.0) (MainStepIterations :type Integer) (ActualMainStep :type "Float (double-precision)") (ActualSubStep :type "Float (double-precision)") (SplineAnchors :type "Array of /Game/ToolsTesting/NewGeneration/S_GoopBaseSplineAnchors Structure") (const_MaxAnchorOffset :type "Float (double-precision)" :default 100.0) (SplinePoints :type "Array of Vector Structure") (LastAnchorNormal :type "Vector Structure") (LastAnchorDirection :type "Vector Structure") (LastSubDirection :type "Vector Structure") (SubStepIterations :type Integer) (LastSubPoint :type "Vector Structure"))
  (bind (_relativepos _thickness) (break `SkeletonPoint` SkeletonPoint1))
  (bind (_relativepos_2 _thickness_2) (break `SkeletonPoint` SkeletonPoint2))
  (bind _substepiterations (`local.SubStepIterations`))
  (bind _returnvalue (`KismetMathLibrary.TransformLocation` (`self.GetTransform`) _relativepos))
  (bind _returnvalue_2 (`KismetMathLibrary.TransformLocation` (`self.GetTransform`) _relativepos_2))
  (bind _returnvalue_3 (- _returnvalue_2 _returnvalue))
  (bind _returnvalue_4 (- (`KismetArrayLibrary.Array_Length` (`local.SplinePoints`)) 1))
  (bind _returnvalue_5 (`KismetMathLibrary.VSize` _returnvalue_3))
  (`KismetMathLibrary.SetRandomStreamSeed` (`local.Stream`) StreamSeed)
  (set `local.Direction` (`KismetMathLibrary.Normal` _returnvalue_3))
  (bind _output_get (set `local.MainStepIterations` (`KismetMathLibrary.FFloor` (/ _returnvalue_5 MainStep))))
  (set `local.ActualMainStep` (/ _returnvalue_5 _output_get))
  (`|ExecutionSequence`
    (:`then_0`
      ;[0.8554 0.6111 1 1 48] Calculating anchor points
      (`KismetArrayLibrary.Array_Add` (`local.SplineAnchors`) (make `/Game/ToolsTesting/NewGeneration/S_GoopBaseSplineAnchors` _returnvalue true))
      (bind _nearestresult (`GeometryScriptLibrary_MeshSpatial.FindNearestPointOnMesh` (`self.SurroundingsRaycastMesh`) (`self.SurroundingsRaycastBVH`) _returnvalue (struct) null)
        (:`Found`
          (set `local.LastAnchorNormal` (`.ReturnValue` (`GeometryScriptLibrary_MeshQueryFunctions.GetTriangleFaceNormal` (`self.SurroundingsRaycastMesh`) (`.TriangleID` (break `GeometryScriptTrianglePoint` _nearestresult)))))
          (set `local.LastAnchorDirection` (`local.Direction`))
          (for _index (range 1 (`local.MainStepIterations`))
            (bind (_nearestresult_2 _returnvalue_6) (`GeometryScriptLibrary_MeshSpatial.FindNearestPointOnMesh` (`self.SurroundingsRaycastMesh`) (`self.SurroundingsRaycastBVH`) (+ (+ (* _index (`local.ActualMainStep`) (`local.Direction`)) _returnvalue) (* (`KismetMathLibrary.Normal` (`KismetMathLibrary.Cross_VectorVector` (`local.LastAnchorDirection`) (`local.LastAnchorNormal`))) (`KismetMathLibrary.RandomFloatInRangeFromStream` (`local.Stream`) -20.0 20.0))) (struct) null)
              (:`Found`
                (set `local.LastAnchorNormal` (`.ReturnValue` (`GeometryScriptLibrary_MeshQueryFunctions.GetTriangleFaceNormal` _returnvalue_6 (`.TriangleID` (break `GeometryScriptTrianglePoint` _nearestresult_2)))))
                (set `local.LastAnchorDirection` (`KismetMathLibrary.Normal` (- _returnvalue_2 (`.Position` (break `GeometryScriptTrianglePoint` _nearestresult_2)))))
                (`KismetArrayLibrary.Array_Add` (`local.SplineAnchors`) (make `/Game/ToolsTesting/NewGeneration/S_GoopBaseSplineAnchors` (`.Position` (break `GeometryScriptTrianglePoint` _nearestresult_2)) true)))))
          (`KismetArrayLibrary.Array_Add` (`local.SplineAnchors`) (make `/Game/ToolsTesting/NewGeneration/S_GoopBaseSplineAnchors` _returnvalue_2 true)))))
    (:`then_1`
      (`KismetArrayLibrary.Array_Add` (`local.SplinePoints`) _returnvalue)
      (for _index_2 (range 1 (`KismetArrayLibrary.Array_Length` (`local.SplineAnchors`)))
        (bind _output_potentialanchorworldposition (break `/Game/ToolsTesting/NewGeneration/S_GoopBaseSplineAnchors` (`|GetArrayItem` (`local.SplineAnchors`) (- _index_2 1))))
        (set `local.LastSubPoint` _output_potentialanchorworldposition)
        (bind _output_potentialanchorworldposition_2 (break `/Game/ToolsTesting/NewGeneration/S_GoopBaseSplineAnchors` (`|GetArrayItem` (`local.SplineAnchors`) _index_2)))
        (bind _returnvalue_7 (- _output_potentialanchorworldposition_2 _output_potentialanchorworldposition))
        (set `local.LastSubDirection` (`KismetMathLibrary.Normal` _returnvalue_7))
        (bind _returnvalue_8 (`KismetMathLibrary.VSize` _returnvalue_7))
        (bind _output_get_2 (set `local.SubStepIterations` (`KismetMathLibrary.FFloor` (/ _returnvalue_8 SubStep))))
        (set `local.ActualSubStep` (/ _returnvalue_8 _output_get_2))
        (for _index_3 (range 1 _substepiterations)
          (bind _returnvalue_9 (+ (`local.LastSubPoint`) (* (/ (`KismetMathLibrary.Vector_Distance` _output_potentialanchorworldposition_2 (`local.LastSubPoint`)) (- _substepiterations _index_3)) (`local.LastSubDirection`))))
          (bind _nearestresult_3 (`GeometryScriptLibrary_MeshSpatial.FindNearestPointOnMesh` (`self.SurroundingsRaycastMesh`) (`self.SurroundingsRaycastBVH`) _returnvalue_9 (struct) null)
            (:`Found`
              (if (>= (`KismetMathLibrary.Vector_Distance` (`.Position` (break `GeometryScriptTrianglePoint` _nearestresult_3)) _returnvalue_9) 1.0)
                (bind _returnvalue_10 (`KismetMathLibrary.MakeVector` (.x _returnvalue_9) (.y _returnvalue_9) (- (.z _returnvalue_9) (* SubStep Gravity))))
                (`self.DrawDebugLineIf` (`local.DebugDraw`) _returnvalue_10 (`local.LastSubPoint`) (struct :`R` 0.456411 :`G` 0.401978 :`B` 1.0 :`A` 1.0) 999.0 1.0)
                (set `local.LastSubPoint` _returnvalue_10)
                (else
                  (`self.DrawDebugLineIf` (`local.DebugDraw`) _returnvalue_9 (`local.LastSubPoint`) (struct :`R` 1.0 :`G` 0.130136 :`B` 0.07036 :`A` 1.0) 999.0 1.0)
                  (set `local.LastSubPoint` _returnvalue_9)))
              (`KismetArrayLibrary.Array_Add` (`local.SplinePoints`) (`local.LastSubPoint`))
              (set `local.LastSubDirection` (`KismetMathLibrary.Normal` (- _output_potentialanchorworldposition_2 (`local.LastSubPoint`))))))))
      (`KismetArrayLibrary.Array_Add` (`local.SplinePoints`) _returnvalue_2)
      (bind _returnvalue_11 (`AddComponent|NODE_AddSplineComponent-4`))
      (`|ExecutionSequence`
        (:`then_0`
          (`SplineComponent.SetSplinePoints` _returnvalue_11 (`local.SplinePoints`) "World" true)
          (for _index_4 (range (+ _returnvalue_4 1))
            (`SplineComponent.SetScaleAtSplinePoint` _returnvalue_11 _index_4 (`KismetMathLibrary.Conv_DoubleToVector` (* (`KismetMathLibrary.Lerp` _thickness _thickness_2 (/ _index_4 _returnvalue_4)) 5.0)) true)))
        (:`then_1`
          (return _returnvalue_11))))))

(fn `MakeMeshFromSpline`
  (params (Spline :type "SplineComponent Object Reference"))
  (returns (ResultingMesh :type "DynamicMesh Object Reference"))
  (locals (Brush :type "GeometryScriptPolyPath Structure"))
  (bind _returnvalue (`GeometryScriptLibrary_PolyPathFunctions.CreateCirclePath2D` (0.0 0.0) 1.0 12))
  (set `local.Brush` _returnvalue)
  (bind _frames (`GeometryScriptLibrary_PolyPathFunctions.SampleSplineToTransforms` Spline (make `GeometryScriptSplineSamplingOptions` (`SplineComponent.GetNumberOfSplinePoints` Spline) 1.0 "UniformDistance" "World")))
  (bind _returnvalue_2 (`self.AllocateComputeMesh`))
  (bind _returnvalue_3 (`GeometryScriptLibrary_MeshPrimitiveFunctions.AppendSweepPolygon` _returnvalue_2 (struct) (struct) (`GeometryScriptLibrary_PolyPathFunctions.Conv_GeometryScriptPolyPathToArrayOfVector2D` (`local.Brush`)) _frames false true 1.0 1.0 0.0 null))
  (return _returnvalue_3))

(fn `PercentageToCentre`
  (params (PathLength :type "Float (double-precision)") (Value :type "Float (double-precision)"))
  (returns (Alpha :type "Float (double-precision)"))
  (return (- 1.0 (`KismetMathLibrary.Abs` (- (* (/ PathLength Value) 2.0) 1.0)))))

(fn `SetVisibilityOfSurroundingGeometry`
  (params (Visibility :type Boolean))
  (for _array_element (`self.SurroundingMeshes`)
    (`SceneComponent.SetVisibility` (`StaticMeshActor.StaticMeshComponent` _array_element) Visibility false)))

(fn `UserConstructionScript`
  (bind _returnvalue (`BaseDynamicMeshComponent.GetDynamicMesh` (`self.DynamicMeshComponent`)))
  (set `self.TargetMesh` _returnvalue))