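; BP_WorldGeometryCache is a tool-testing Blueprint that caches the geometry of a set of target actors as one combined mesh with a BVH, apparently for raycast queries.
; UpdateRaycastMesh uses Geometry Script to copy each actor's root component mesh in world space into a pooled compute mesh, append it to RaycastMesh, then release the temporary mesh.
; BuildBVH separately builds and stores the BVH from that merged mesh.
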(fn `BuildBVH`
  (bind _outputbvh (`GeometryScriptLibrary_MeshSpatial.BuildBVHForMesh` (`self.RaycastMesh`) null))
  (set `self.RaycastMeshBVH` _outputbvh))

(fn `UpdateRaycastMesh`
  (bind _returnvalue (`self.AllocateComputeMesh`))
  (set `self.RaycastMesh` _returnvalue)
  (for _array_element (`self.TargetActors`)
    (bind _returnvalue_2 (`self.AllocateComputeMesh`))
    (bind (_localtoworld _returnvalue_3) (`GeometryScriptLibrary_SceneUtilityFunctions.CopyMeshFromComponent` (`Actor.RootComponent` _array_element) _returnvalue_2 (struct) true null)
      (:`Failure`
        _)
      (:`Success`
        (`GeometryScriptLibrary_MeshBasicEditFunctions.AppendMesh` (`self.RaycastMesh`) _returnvalue_3 (struct) false (struct :`CombineMode` "EnableAllMatching") null)))
    (`self.ReleaseComputeMesh` _returnvalue_2)))

(fn `UserConstructionScript`)