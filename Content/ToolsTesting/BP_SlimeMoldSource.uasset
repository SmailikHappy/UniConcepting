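; Slime mold actor that builds a procedural dynamic mesh along a skeleton of Points and Lines using Geometry Script.
; GenerateMesh clears the mesh, then splits each line into randomly offset cylinder segments from a fixed-seed stream, giving repeatable fractured strands.
; Optional retopology fuses them with SDF morphology, tessellation and smoothing, then rebuilds planar UVs and normals.
; The mesh is moved into actor space and given the main material, which SetTranslucensy can swap.
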(event `self.ReceiveBeginPlay`)

(event `ClearMesh`
  (bind (_triangleidlist _bhastriangleidgaps _returnvalue) (`GeometryScriptLibrary_MeshQueryFunctions.GetAllTriangleIDs` (`self.TargetMesh`)))
  (`GeometryScriptLibrary_MeshBasicEditFunctions.DeleteTrianglesFromMesh` _returnvalue _triangleidlist))

(event `GenerateMesh`
  (params (RetopologyInfo :type "/Game/ToolsTesting/MeshEditing/SRetopologySlimeMoldMesh Structure (by ref)") (ApplyRetopology :type Boolean) (MeshGenerationInfo :type "/Game/ToolsTesting/MeshEditing/SMeshGenerationSlimeMoldMesh Structure"))
  (bind (_gridcellsize _thickness _smothiteration _smothnessalpha _uvscale _uvoffset) (break `/Game/ToolsTesting/MeshEditing/SRetopologySlimeMoldMesh` RetopologyInfo))
  (bind (_gridcellsize_2 _thickness_2 _smothiteration_2 _smothnessalpha_2 _uvscale_2 _uvoffset_2 _tessellationsubdivision) (break `/Game/ToolsTesting/MeshEditing/SRetopologySlimeMoldMesh` RetopologyInfo))
  (`|ExecutionSequence`
    (:`then_0`
      (`self.ClearMesh`)
      (`KismetMathLibrary.SetRandomStreamSeed` (`self.Stream`)))
    (:`then_1`
      (`self.GeneratedGeometry` MeshGenerationInfo))
    (:`then_2`
      ;[1 1 1] Retopologing spawned spheres into a big layer of snow
      (if ApplyRetopology
        (bind _returnvalue (`GeometryScriptLibrary_MeshVoxelFunctions.ApplyMeshMorphology` (`self.TargetMesh`) (make `GeometryScriptMorphologyOptions` (make `GeometryScript3DGridParameters` "GridCellSize" _gridcellsize_2) false (make `GeometryScript3DGridParameters` "GridResolution") "Dilate" _thickness_2) null))
        (bind _returnvalue_2 (`GeometryScriptLibrary_MeshSubdivideFunctions.ApplyPNTessellation` _returnvalue (make `GeometryScriptPNTessellateOptions` true) _tessellationsubdivision null))
        (bind _returnvalue_3 (`GeometryScriptLibrary_MeshDeformFunctions.ApplyIterativeSmoothingToMesh` _returnvalue_2 (struct) (make `GeometryScriptIterativeMeshSmoothingOptions` _smothiteration_2 _smothnessalpha_2) null))
        (bind _returnvalue_4 (`GeometryScriptLibrary_MeshUVFunctions.SetMeshUVsFromPlanarProjection` _returnvalue_3 0 (`KismetMathLibrary.MakeTransform` (0.0 0.0 0.0) (struct) (`KismetMathLibrary.Conv_DoubleToVector` (`KismetMathLibrary.FMax` (.x (`KismetMathLibrary.GetBoxSize` (`GeometryScriptLibrary_MeshQueryFunctions.GetMeshBoundingBox` _returnvalue_3))) (.y (`KismetMathLibrary.GetBoxSize` (`GeometryScriptLibrary_MeshQueryFunctions.GetMeshBoundingBox` _returnvalue_3)))))) (struct) null))
        (bind _returnvalue_5 (`GeometryScriptLibrary_MeshNormalsFunctions.ComputeTangents` _returnvalue_4 (struct) null))
        (bind _returnvalue_6 (`GeometryScriptLibrary_MeshNormalsFunctions.ComputeSplitNormals` _returnvalue_5 (make `GeometryScriptSplitNormalsOptions` true 80.0) (struct) null))
        (bind _returnvalue_7 (`GeometryScriptLibrary_MeshUVFunctions.ScaleMeshUVs` _returnvalue_6 0 _uvscale (0.5 0.5) (struct) null))
        (`GeometryScriptLibrary_MeshUVFunctions.TranslateMeshUVs` _returnvalue_7 0 _uvoffset (struct) null)))
    (:`then_3`
      ;[1 1 1] Setting world transform for final mesh
      (`GeometryScriptLibrary_MeshTransformFunctions.TransformMesh` (`self.TargetMesh`) (`KismetMathLibrary.InvertTransform` (`self.GetTransform`)) true null))
    (:`then_4`
      (`self.AssignMaterials`))))

(event `AssignMaterials`
  (`DynamicMeshComponent.ConfigureMaterialSet` (`self.DynamicMeshComponent`) (`|MakeArray` (`self.MainMaterial`) :!type "MaterialInterface Object Reference")))

(event `SetTranslucensy`
  (params (IsTranslucent :type Boolean) (TranslucentMaterial :type "MaterialInterface Object Reference"))
  (if IsTranslucent
    (`DynamicMeshComponent.ConfigureMaterialSet` (`self.DynamicMeshComponent`) (`|MakeArray` TranslucentMaterial))
    (else
      (`self.AssignMaterials`))))

(fn `GeneratedGeometry`
  (params (MeshGenerationInfo :type "/Game/ToolsTesting/MeshEditing/SMeshGenerationSlimeMoldMesh Structure"))
  (locals (PreviousLocation :type "Vector Structure") (Step :type "Vector Structure") (Direction :type "Vector Structure") (NewLocation :type "Vector Structure"))
  (bind _points (`self.Points`))
  ;[1 1 1] #2
  (for _array_element (`self.Lines`)
    (bind _output (`|GetArrayItem` _points (`.PointIndex1_6_FDCF312941EBE3375DF70D837915F21F` (break `/Game/ToolsTesting/SkeletonEditing/SLine` _array_element))))
    (set `local.PreviousLocation` _output)
    (bind _returnvalue (- (`|GetArrayItem` _points (break `/Game/ToolsTesting/SkeletonEditing/SLine` _array_element)) _output))
    (bind _returnvalue_2 (`KismetMathLibrary.FCeil` (/ (`KismetMathLibrary.VSizeXY` _returnvalue) MeshGenerationInfo_FractureStep_23_62119D654AC54F66B7C8ADA2B932C819)))
    (bind _output_get (set `local.Step` (/ _returnvalue _returnvalue_2)))
    (set `local.Direction` (`KismetMathLibrary.Normal` _output_get))
    (for _index (range 1 (+ _returnvalue_2 1))
      (bind _output_get_2 (set `local.NewLocation` (+ (* _index (`local.Step`)) _output (* (`KismetMathLibrary.Normal` (`KismetMathLibrary.Cross_VectorVector` (`local.Direction`) (`self.PointAverageWorldNormal`))) (`KismetMathLibrary.RandomFloatInRangeFromStream` (`self.Stream`) (* -1.0 MeshGenerationInfo_FractureOffsets_22_5C927CA54180E5CFE73F33B9F9888842) MeshGenerationInfo_FractureOffsets_22_5C927CA54180E5CFE73F33B9F9888842)))))
      (bind _returnvalue_3 (- (`local.PreviousLocation`) _output_get_2))
      (`GeometryScriptLibrary_MeshPrimitiveFunctions.AppendCylinder` (`self.TargetMesh`) (struct) (`KismetMathLibrary.MakeTransform` _output_get_2 (`KismetMathLibrary.MakeRotFromZ` _returnvalue_3)) MeshGenerationInfo_SubjectRadius_20_2AD92F3F4F1BDA1F3E7B3BAF4DAAE7B8 (`KismetMathLibrary.VSize` _returnvalue_3) 12 0 true "Base" null)
      (set `local.PreviousLocation` (`local.NewLocation`)))))

(fn `UserConstructionScript`
  (bind _returnvalue (`BaseDynamicMeshComponent.GetDynamicMesh` (`self.DynamicMeshComponent`)))
  (set `self.TargetMesh` _returnvalue))