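; Geometry Script generated-mesh actor that builds a procedural snow layer over selected mesh actors.
; Generatemeshcache merges their world-space meshes and builds a BVH for downward grid raycasts.
; Hits on sufficiently upward-facing triangles receive normal-aligned, Z-scaled sphere boxes.
; With Remesh enabled, morphology and smoothing fuse these into snow, which gets planar UVs, PN tessellation and texture displacement before conversion to actor space.
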(event `Generate mesh cache`
  (`|ExecutionSequence`
    (:`then_0`
      (bind _returnvalue (`self.AllocateComputeMesh`))
      (set `self.Raycast Mesh Actors` _returnvalue)
      ;[1 1 1] Add all the selected meshes to a one single one
      (for _array_element (`self.MeshesToAddSnowTo`)
        (bind _returnvalue_2 (`self.AllocateComputeMesh`))
        (`|ExecutionSequence`
          (:`then_0`
            (bind (_localtoworld _returnvalue_3) (`GeometryScriptLibrary_SceneUtilityFunctions.CopyMeshFromComponent` (`Actor.RootComponent` _array_element) _returnvalue_2 (struct) true null)
              (:`Success`
                (`GeometryScriptLibrary_MeshBasicEditFunctions.AppendMesh` (`self.Raycast Mesh Actors`) _returnvalue_3 (struct) false (struct :`CombineMode` "EnableAllMatching") null))))
          (:`then_1`
            (`self.ReleaseComputeMesh` _returnvalue_2)))))
    (:`then_1`
      ;[1 1 1] Calculating BVH
      (bind _outputbvh (`GeometryScriptLibrary_MeshSpatial.BuildBVHForMesh` (`self.Raycast Mesh Actors`) null))
      (set `self.Output BVH` _outputbvh))))

(event `self.OnRebuildGeneratedMesh`
  (params (TargetMesh :type "DynamicMesh Object Reference"))
  (bind _grid_spacing (`self.Grid Spacing`))
  (bind _returnvalue (`GeometryScriptLibrary_MeshQueryFunctions.GetMeshBoundingBox` (`self.Raycast Mesh Actors`)))
  (set `self.Target Mesh` TargetMesh)
  (if (`self.Generate snow?`)
    (`|ExecutionSequence` :!label _label
      (:`then_0`
        ;[1 1 1] Raycasting the model
        ;;[1 1 1] Contructing a grid of rays
        (for _index (range (+ (`KismetMathLibrary.Round` (/ (- (.x (`.Max` (break `Box` _returnvalue))) (.x (break `Box` _returnvalue))) _grid_spacing)) 1))
          (for _index_2 (range (+ (`KismetMathLibrary.Round` (/ (- (.y (`.Max` (break `Box` _returnvalue))) (.y (break `Box` _returnvalue))) _grid_spacing)) 1))
            (bind (_hitresult _returnvalue_2) (`GeometryScriptLibrary_MeshSpatial.FindNearestRayIntersectionWithMesh` (`self.Raycast Mesh Actors`) (`self.Output BVH`) (`KismetMathLibrary.MakeVector` (+ (.x (break `Box` _returnvalue)) (* (`self.Grid Spacing`) _index)) (+ (.y (break `Box` _returnvalue)) (* (`self.Grid Spacing`) _index_2)) (+ (- (.z (`.Max` (break `Box` _returnvalue))) (.z (break `Box` _returnvalue))) 1000.0)) (0.0 0.0 -1.0) (struct) null)
              (:`Found`
                (if (`self.UseAltSnowCoverageMethod?`)
                  (bind (_bisvalidtriangle _returnvalue_3) (`GeometryScriptLibrary_MeshQueryFunctions.GetTriangleFaceNormal` _returnvalue_2 (`.HitTriangleID` (break `GeometryScriptRayHitResult` _hitresult))))
                  (if (>= (.z _returnvalue_3) (`KismetMathLibrary.Abs` (- (`self.Snow Coverage`) 1.0)))
                    ;;[1 1 1] Placing a sphere at a ray-cast position
                    (`GeometryScriptLibrary_MeshPrimitiveFunctions.AppendSphereBox` (`self.Target Mesh`) (struct) (`KismetMathLibrary.MakeTransform` (`.HitPosition` (break `GeometryScriptRayHitResult` _hitresult)) (`KismetMathLibrary.MakeRotFromZ` _returnvalue_3) (`KismetMathLibrary.MakeVector` 1.0 1.0 (`self.Snow Sphere Scale`))) (`self.Sphere Radius`) 6 6 6 "Center" null :!label _label_2))
                  (elif (== _returnvalue_3 (0.0 0.0 1.0) :`ErrorTolerance` (`self.Snow Coverage`))
                    (goto _label_2))))))))
      (:`then_1`
        ;[1 1 1] Retopologing spawned spheres into a big layer of snow
        (if (`self.Remesh`)
          (bind _returnvalue_4 (`GeometryScriptLibrary_MeshVoxelFunctions.ApplyMeshMorphology` (`self.Target Mesh`) (make `GeometryScriptMorphologyOptions` (make `GeometryScript3DGridParameters` "GridCellSize" (`self.Grid Cell Size`)) false (make `GeometryScript3DGridParameters` "GridResolution") "Dilate" (`self.Snow Thickness`)) null))
          (bind _returnvalue_5 (`GeometryScriptLibrary_MeshDeformFunctions.ApplyIterativeSmoothingToMesh` _returnvalue_4 (struct) (make `GeometryScriptIterativeMeshSmoothingOptions` (`self.Smooth Iterations`)) null))
          (bind _returnvalue_6 (`GeometryScriptLibrary_MeshUVFunctions.SetMeshUVsFromPlanarProjection` _returnvalue_5 0 (`KismetMathLibrary.MakeTransform` (0.0 0.0 0.0) (struct) (`KismetMathLibrary.Conv_DoubleToVector` (`KismetMathLibrary.FMax` (.x (`KismetMathLibrary.GetBoxSize` (`GeometryScriptLibrary_MeshQueryFunctions.GetMeshBoundingBox` _returnvalue_5))) (.y (`KismetMathLibrary.GetBoxSize` (`GeometryScriptLibrary_MeshQueryFunctions.GetMeshBoundingBox` _returnvalue_5)))))) (struct) null))
          (bind _returnvalue_7 (`GeometryScriptLibrary_MeshNormalsFunctions.ComputeTangents` _returnvalue_6 (struct) null))
          (bind _returnvalue_8 (`GeometryScriptLibrary_MeshNormalsFunctions.ComputeSplitNormals` _returnvalue_7 (make `GeometryScriptSplitNormalsOptions` true 80.0) (struct) null))
          (bind _returnvalue_9 (`GeometryScriptLibrary_MeshUVFunctions.ScaleMeshUVs` _returnvalue_8 0 (`self.UVScale`) (0.5 0.5) (struct) null))
          (`GeometryScriptLibrary_MeshUVFunctions.TranslateMeshUVs` _returnvalue_9 0 (`self.UVOffset`) (struct) null)
          (`GeometryScriptLibrary_MeshSubdivideFunctions.ApplyPNTessellation` (`self.Target Mesh`) (make `GeometryScriptPNTessellateOptions` true) (`self.SubdivisionAmount`) null)))
      (:`then_2`
        (if (`self.Remesh`)
          ;[1 1 1] Creating some extra details to the displacement of some snow
          (bind _returnvalue_10 (`GeometryScriptLibrary_MeshDeformFunctions.ApplyDisplaceFromTextureMap` (`self.Target Mesh`) (`self.Displacement Texture`) (struct) (make `GeometryScriptDisplaceFromTextureOptions` (`self.Displacement Amount`) (1.0 1.0) (0.0 0.0) (`self.Displacement Center`) (`self.Displacement Image Channel`)) 0 null))
          (bind _returnvalue_11 (`GeometryScriptLibrary_MeshNormalsFunctions.ComputeTangents` _returnvalue_10 (struct) null))
          (`GeometryScriptLibrary_MeshNormalsFunctions.ComputeSplitNormals` _returnvalue_11 (make `GeometryScriptSplitNormalsOptions` true 90.0) (struct) null)))
      (:`then_3`
        ;[1 1 1] Setting world transform for final mesh
        (`GeometryScriptLibrary_MeshTransformFunctions.TransformMesh` (`self.Target Mesh`) (`KismetMathLibrary.InvertTransform` (`self.GetTransform`)) true null)))))

(event `Generate Mesh`
  (set `self.Generate snow?` true)
  (goto _label))

(fn `UserConstructionScript`)