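; Slime mold generated-mesh actor that scatters small boxes over level geometry using Geometry Script.
; Construction script finds the level's single BP_GeometryCache, which supplies a raycast mesh and BVH, refreshed by UpdateGeometryCache.
; Regeneration clears the mesh, then casts seeded random downward rays within the cache's XY bounds, appending a box at each hit.
; The inverse actor transform then converts the world-space result into local space.
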(event `UpdateGeometryCache`
  (bind _geometrycache (`self.GeometryCache`))
  (`/Game/LivingDecays/BP_GeometryCache.UpdateRaycastMesh` _geometrycache)
  (`/Game/LivingDecays/BP_GeometryCache.BuildBVH` _geometrycache))

(event `self.OnRebuildGeneratedMesh`
  (params (TargetMesh :type "DynamicMesh Object Reference"))
  (set `self.Target Mesh` TargetMesh)
  (`self.(Re)GenerateMesh`))

(event `(Re)GenerateMesh`
  (bind _streamrandom (`self.StreamRandom`))
  (bind _returnvalue (`GeometryScriptLibrary_MeshQueryFunctions.GetMeshBoundingBox` (`/Game/LivingDecays/BP_GeometryCache.RaycastMesh` (`self.GeometryCache`))))
  (`self.ClearTargetMesh`)
  (`/Engine/EditorBlueprintResources/StandardMacros.IsValid` (`self.GeometryCache`)
    (:`Is Valid`
      (`|ExecutionSequence`
        (:`then_0`
          (`self.SetDefaults`))
        (:`then_1`
          (for _ (range 201)
            (bind _hitresult (`GeometryScriptLibrary_MeshSpatial.FindNearestRayIntersectionWithMesh` (`/Game/LivingDecays/BP_GeometryCache.RaycastMesh` (`self.GeometryCache`)) (`/Game/LivingDecays/BP_GeometryCache.RaycastMeshBVH` (`self.GeometryCache`)) (`KismetMathLibrary.MakeVector` (`KismetMathLibrary.RandomFloatInRangeFromStream` _streamrandom (.x (break `Box` _returnvalue)) (.x (`.Max` (break `Box` _returnvalue)))) (`KismetMathLibrary.RandomFloatInRangeFromStream` _streamrandom (.y (break `Box` _returnvalue)) (.y (`.Max` (break `Box` _returnvalue)))) 10000.0) (0.0 0.0 -1.0) (struct) null)
              (:`Found`
                (`GeometryScriptLibrary_MeshPrimitiveFunctions.AppendBox` (`self.Target Mesh`) (struct) (`KismetMathLibrary.MakeTransform` (`.HitPosition` (break `GeometryScriptRayHitResult` _hitresult))) 10.0 10.0 10.0 0 0 0 "Base" null)))))
        (:`then_2`
          (`self.PositioningTargetMesh`))))))

(event `DeleteMesh`
  (`self.ClearTargetMesh`))

(fn `ClearTargetMesh`
  (bind (_triangleidlist _bhastriangleidgaps _returnvalue) (`GeometryScriptLibrary_MeshQueryFunctions.GetAllTriangleIDs` (`self.Target Mesh`)))
  (`GeometryScriptLibrary_MeshBasicEditFunctions.DeleteTrianglesFromMesh` _returnvalue _triangleidlist))

(fn `PositioningTargetMesh`
  (`GeometryScriptLibrary_MeshTransformFunctions.TransformMesh` (`self.Target Mesh`) (`KismetMathLibrary.InvertTransform` (`self.GetTransform`)) true null))

(fn `SetDefaults`
  (set `self.StreamRandom` (`KismetMathLibrary.MakeRandomStream` (`self.SeedRandom`))))

(fn `UserConstructionScript`
  (bind _outactors (`GameplayStatics.GetAllActorsOfClass` "/Game/LivingDecays/BP_GeometryCache.BP_GeometryCache_C"))
  (if (== (`KismetArrayLibrary.Array_Length` _outactors) 1)
    (set `self.GeometryCache` (`|GetArrayItem` _outactors))
    (else
      (`KismetSystemLibrary.PrintString` "Wrong number of BP_GeometryCaches on the level")
      (set `self.GeometryCache` null))))