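; Light beam actor that fires along its up vector and fits a visible cylinder and point light to the surfaces it hits.
; Four visibility traces at the beam's edges find the furthest hit, falling back to max length on a miss.
; That distance scales and centers the cylinder and places the light just short of the end.
; It updates in the construction script and every Tick, drawing debug traces.
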(event `self.ReceiveTick`
  (params (DeltaSeconds :type "Float (single-precision)"))
  (`self.SetTraceOffsets`)
  (`self.UpdateLightBeam` "ForOneFrame"))

(fn `SetTraceOffsets`
  (bind _defaultsceneroot (`self.DefaultSceneRoot`))
  (bind _returnvalue (* (`SceneComponent.GetRightVector` _defaultsceneroot) (* (`self.BeamDiameter`) 0.5)))
  (bind _returnvalue_2 (* (`SceneComponent.GetForwardVector` _defaultsceneroot) (* (`self.BeamDiameter`) 0.5)))
  (`KismetArrayLibrary.Array_Set` (`self.TraceOffsets`) 0 _returnvalue true)
  (`KismetArrayLibrary.Array_Set` (`self.TraceOffsets`) 1 (* _returnvalue -1.0) true)
  (`KismetArrayLibrary.Array_Set` (`self.TraceOffsets`) 2 _returnvalue_2 true)
  (`KismetArrayLibrary.Array_Set` (`self.TraceOffsets`) 3 (* _returnvalue_2 -1.0) true))

(fn `UpdateLightBeam`
  (params (DrawDebugType :type "EDrawDebugTrace Enum" :default "ForOneFrame"))
  (bind _returnvalue (`SceneComponent.K2_GetComponentLocation` (`self.DefaultSceneRoot`)))
  (bind _returnvalue_2 (`SceneComponent.K2_GetComponentLocation` (`self.DefaultSceneRoot`)))
  (bind _returnvalue_3 (* (`self.FurthestDistance`) (`self.TraceNormal`)))
  (bind _returnvalue_4 (* (`self.BeamDiameter`) 0.01))
  (set `self.TraceNormal` (`KismetMathLibrary.Normal` (`SceneComponent.GetUpVector` (`self.DefaultSceneRoot`))))
  (set `self.FurthestDistance` 0.0)
  (for _array_element (`self.TraceOffsets`)
    (bind (_outhit _returnvalue_5) (`KismetSystemLibrary.LineTraceSingle` :`Start` (+ _array_element _returnvalue_2) :`End` (+ _array_element (+ _returnvalue_2 (* (`self.TraceNormal`) (`self.BeamMaxLength`)))) :`TraceChannel` "TraceTypeQuery1" :`DrawDebugType` DrawDebugType))
    (if _returnvalue_5
      (bind (_bblockinghit _binitialoverlap _time _distance) (`GameplayStatics.BreakHitResult` _outhit))
      (if (> _distance (`self.FurthestDistance`))
        (set `self.FurthestDistance` _distance))
      (else
        (set `self.FurthestDistance` (`self.BeamMaxLength`)) ; we didn't hit anything, so go for max
      )))
  (`SceneComponent.K2_SetWorldLocation` (`self.PointLight`) (+ (+ (* (`self.TraceNormal`) -100.0) _returnvalue_3) _returnvalue) false false)
  (`SceneComponent.SetRelativeScale3D` (`self.VisibleLightBeamCylinder`) (`KismetMathLibrary.MakeVector` _returnvalue_4 _returnvalue_4 (`KismetMathLibrary.VSize` (/ _returnvalue_3 100.0))))
  (`SceneComponent.K2_SetWorldLocation` (`self.VisibleLightBeamCylinder`) (+ (* _returnvalue_3 0.5) _returnvalue) false false))

(fn `UserConstructionScript`
  (`self.SetTraceOffsets`)
  (`self.UpdateLightBeam` "ForDuration"))